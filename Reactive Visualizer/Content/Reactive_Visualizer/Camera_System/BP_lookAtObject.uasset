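; Look-at object for the reactive visualizer's camera system that glides toward a target actor chosen by MIDI.
; BeginPlay selects the first entry of TargetArray, and Tick interpolates the actor's location toward the active target at InterpSpeed.
; The router's MIDI note event, filtered to the camera channel, maps notes 12 to 23 onto array indices to switch the active target.
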(event `self.ReceiveBeginPlay`
  ;[1 1 1] begin play
  (`self.setFirstTargetToZero`))

(event `self.ReceiveTick`
  (params (DeltaSeconds :type "Float (single-precision)"))
  (bind _activetarget (`self.activeTarget`))
  ;[1 1 1] event tick
  (`/Engine/EditorBlueprintResources/StandardMacros.IsValid` _activetarget
    (:`Is Valid`
      (`self.K2_SetActorLocation` (`KismetMathLibrary.VInterpTo` (`self.K2_GetActorLocation`) (`self.K2_GetActorLocation` _activetarget) (`self.Delta Time`) (`self.Interp Speed`))))))

(event `self.routerReference.onMidiNote`
  (params (trackAddress :type Integer) (noteValue :type Integer))
  ;[1 1 1] set camera channel
  (if (== trackAddress (`self.cameraChannel`))
    (bind _output_get (set `self.noteValue` noteValue))
    ;[1 1 1] define note range
    (if (`KismetMathLibrary.InRange_IntInt` _output_get 12 23)
      ;[1 1 1] select active target on corresponding midi note
      (bind _output_get_2 (set `self.targetArray` (`self.targetArray`)))
      (for (_array_element _array_index) _output_get_2 :!label _label
        (if (== _array_index (- (`self.noteValue`) 12))
          (set `self.activeTarget` _array_element)
          (`self.breakLoop`))))))

(event `breakLoop`
  ;[1 1 1] select active target on corresponding midi note
  (goto _label :!via `Break`))

(fn `setFirstTargetToZero`
  (set `self.activeTarget` (`|GetArrayItem` (`self.targetArray`))))

(fn `UserConstructionScript`)