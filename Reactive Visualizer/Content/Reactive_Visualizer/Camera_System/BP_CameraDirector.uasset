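; BP_CameraDirector switches cameras and triggers camera shakes from MIDI notes received through an OSC router.
; Notes on its camera channel are split by range: 0-11 select from CameraArray with an eased view-target blend, while 24-35 hold shake behaviours.
; The first five behaviour notes play low, high, slow, roll or FOV shakes at the active camera.
; On play it activates the first camera, optionally setting the view and adding constant subtle shake.
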(event `setActiveCamera`
  (params (`active camera` :type "CameraActor Object Reference"))
  ;[1 1 1] set active camera
  (set `self.ActiveCamera` `active camera`))

(event `self.ReceiveBeginPlay`
  ;[1 1 1] on level start
  (if (`self.subtleCameraMovement`)
    (`GameplayStatics.PlayWorldCameraShake` "/Game/Reactive_Visualizer/Camera_System/Camera_Shakes/BP_camShakeConstant1.BP_camShakeConstant1_C" (0.0 0.0 0.0) 0.0 10000.0))
  (`self.setActiveCamera` (`|GetArrayItem` (`self.cameraArray`)))
  (if (`self.should set view on play`)
    (`self.setViewToActiveCam`)))

(event `self.oscRouterRef.onMidiNote`
  (params (trackAddress :type Integer) (noteValue :type Integer))
  ;[1 1 1] on Midi Note
  (bind _output_get (`self.setChannelAndNoteValue` trackAddress noteValue))
  ;[1 1 1] define note ranges
  (`self.defineNoteRanges` _output_get
    (:`0-11`
      ;[1 1 1] set Active Camera from Camera Array (range 0-11)
      (for (_array_element _array_index) (`self.cameraArray`) :!label _label
        (if (== _array_index (`self.noteValue`))
          (`self.setActiveCamera` _array_element)
          (`self.setViewToActiveCam`)
          (`self.breakViewLoop`))))
    (:`24-35`
      ;[1 1 1] behaviours (range 24-35)
      (switch `int` (- (`self.noteValue`) 24)
        (:`0`
          (`self.shakePulseLo`))
        (:`1`
          (`self.shakePulseHi`))
        (:`2`
          (`self.shakePulseSlow`))
        (:`3`
          (`self.shakePulseRoll`))
        (:`4`
          (`self.shakePulseFOV`))))))

(event `breakViewLoop`
  ;[1 1 1] set Active Camera from Camera Array (range 0-11)
  (goto _label :!via `Break`))

(event `setViewToActiveCam`
  ;[1 1 1] set view to active camera
  (`PlayerController.SetViewTargetWithBlend` (`GameplayStatics.GetPlayerController` 0) (`self.ActiveCamera`) (`self.blendTime`) "VTBlend_EaseInOut" (`self.easeIn/Out`) false))

(fn `count1`
  (set `self.counter` (+ (`self.counter`) 1.0)))

(fn `followTarget`
  (set `self.lookAtVector` (`self.K2_GetActorLocation` (`self.lookAtTarget`))))

(fn `setFirstTargetToZero`
  (returns (Output :type "/Game/Reactive_Visualizer/Camera_System/BP_Target_0 Object Reference"))
  (bind _outactors (`GameplayStatics.GetAllActorsOfClass` "/Game/Reactive_Visualizer/Camera_System/BP_Target_0.BP_Target_0_C"))
  (return (`|GetArrayItem` _outactors)))

(fn `setLookatVector1`
  (bind _lookattarget (`self.lookAtTarget`))
  (`/Engine/EditorBlueprintResources/StandardMacros.IsValid` _lookattarget
    (:`Is Valid`
      (set `self.lookAtVector` (`self.K2_GetActorLocation` _lookattarget)))))

(fn `setRootTransform1`
  (set `self.originalRootVector` (+ (`SceneComponent.K2_GetComponentLocation` (`self.DefaultSceneRoot`)) (0.0 0.0 0.0))))

(fn `shakePulseFOV`
  (`GameplayStatics.PlayWorldCameraShake` "/Game/Reactive_Visualizer/Camera_System/Camera_Shakes/BP_camShakeFOV.BP_camShakeFOV_C" (`self.K2_GetActorLocation` (`self.ActiveCamera`)) 0.0 500.0))

(fn `shakePulseHi`
  (`GameplayStatics.PlayWorldCameraShake` "/Game/Reactive_Visualizer/Camera_System/Camera_Shakes/BP_camShakeHi.BP_camShakeHi_C" (`self.K2_GetActorLocation` (`self.ActiveCamera`)) 0.0 500.0))

(fn `shakePulseLo`
  (`GameplayStatics.PlayWorldCameraShake` "/Game/Reactive_Visualizer/Camera_System/Camera_Shakes/BP_camShakeLo.BP_camShakeLo_C" (`self.K2_GetActorLocation` (`self.ActiveCamera`)) 0.0 500.0))

(fn `shakePulseRoll`
  (`GameplayStatics.PlayWorldCameraShake` "/Game/Reactive_Visualizer/Camera_System/Camera_Shakes/BP_camShakeRoll.BP_camShakeRoll_C" (`self.K2_GetActorLocation` (`self.ActiveCamera`)) 0.0 500.0))

(fn `shakePulseSlow`
  (`GameplayStatics.PlayWorldCameraShake` "/Game/Reactive_Visualizer/Camera_System/Camera_Shakes/BP_camShakeSlow.BP_camShakeSlow_C" (`self.K2_GetActorLocation` (`self.ActiveCamera`)) 0.0 500.0))

(fn `UserConstructionScript`)